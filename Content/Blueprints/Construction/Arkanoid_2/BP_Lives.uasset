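; BP_Lives is an Arkanoid life counter that tracks the Lives value and displays it through its Count text.
; On BeginPlay it shows the starting value and binds handlers to its DecreaseLives and EncreaseLives event dispatchers.
; Each handler changes Lives by one and refreshes the text through the SetLivesText function, with no limit checks or game-over logic.
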(event `self.ReceiveBeginPlay`
  (`self.SetLivesText` (`self.Lives`))
  (add `self.decreaseLives` (delegate `onDecreaseLives`))
  (add `self.encreaseLives` (delegate `onEncreaseLives`)))

(event `onDecreaseLives`
  (bind _output_get (set `self.Lives` (- (`self.Lives`) 1)))
  (`self.SetLivesText` _output_get))

(event `onEncreaseLives`
  (bind _output_get (set `self.Lives` (+ (`self.Lives`) 1)))
  (`self.SetLivesText` _output_get))

(fn `SetLivesText`
  (params (Lives :type Integer))
  (`TextRenderComponent.K2_SetText` (`self.Count`) (`KismetTextLibrary.Conv_IntToText` Lives)))

(fn `UserConstructionScript`)