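; BP_Simple_Block is an Arkanoid brick that takes damage from ball hits and can drop a bonus.
; The Hit event calls BallHit, which ignores anything but BP_Ball, decrements Lives and swaps the hit component's material.
; At zero Lives it destroys that component rather than the actor, with a small chance to call TakeBonus.
; TakeBonus spawns a random ball, wall or lives bonus at the SpawnBonus transform.
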(event `self.ReceiveHit`
  (params (MyComp :type "PrimitiveComponent Object Reference") (Other :type "Actor Object Reference") (OtherComp :type "PrimitiveComponent Object Reference") (bSelfMoved :type Boolean) (HitLocation :type "Vector Structure") (HitNormal :type "Vector Structure") (NormalImpulse :type "Vector Structure") (Hit :type "HitResult Structure (by ref)"))
  (`self.Ball Hit` Other MyComp))

(fn `Ball Hit`
  (params (Ball :type "Actor Object Reference") (Block :type "PrimitiveComponent Object Reference"))
  (cast `/Game/Blueprints/Construction/BP_Ball` Ball)
  (set `self.Lives` (- (`self.Lives`) 1))
  (`PrimitiveComponent.SetMaterial` Block 0 "/Game/Environment/Materials/M_Arkanoid_Items_2.M_Arkanoid_Items_2")
  (if (<= (`self.Lives`) 0)
    (`ActorComponent.K2_DestroyComponent` Block)
    (if (`KismetMathLibrary.RandomBoolWithWeight` 0.1)
      (`self.Take Bonus`))))

(fn `Take Bonus`
  (bind _returnvalue (`SceneComponent.K2_GetComponentToWorld` (`self.Spawn Bonus`)))
  (switch `int` (`KismetMathLibrary.RandomIntegerInRange` 0 2)
    (:`0`
      (`|SpawnActorFromClass` "/Game/Blueprints/Construction/Arkanoid_2/BP_Bonus_Ball.BP_Bonus_Ball_C" _returnvalue "AlwaysSpawn" "OverrideRootScale" null null))
    (:`1`
      (`|SpawnActorFromClass` "/Game/Blueprints/Construction/Arkanoid_2/BP_Bonus_Wall.BP_Bonus_Wall_C" _returnvalue "AlwaysSpawn" "OverrideRootScale" null null))
    (:`2`
      (`|SpawnActorFromClass` "/Game/Blueprints/Construction/Arkanoid_2/BP_Bonus_Lives.BP_Bonus_Lives_C" _returnvalue "AlwaysSpawn" "OverrideRootScale" null null))))

(fn `UserConstructionScript`)