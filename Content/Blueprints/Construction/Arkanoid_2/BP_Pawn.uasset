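; Player paddle pawn for an Arkanoid-style game that moves sideways and spawns the ball.
; Left and right axis inputs apply swept, fixed-step world offsets along Y, without delta-time scaling.
; On BeginPlay, SpawnBall creates a BP_Ball at the capsule's transform, stores the reference and binds a delegate to the ball's OnDead event.
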(event `self.ReceiveBeginPlay`
  (`self.SpawnBall`))

(event `InputAxis|MoveRight`
  (params (AxisValue :type "Float (single-precision)"))
  (if (> AxisValue 0.0)
    (`self.K2_AddActorWorldOffset` (0.0 30.0 0.0) true)))

(event `InputAxis|MoveLeft`
  (params (AxisValue :type "Float (single-precision)"))
  (if (< AxisValue 0.0)
    (`self.K2_AddActorWorldOffset` (0.0 -30.0 0.0) true)))

(fn `SpawnBall`
  (bind _returnvalue (`|SpawnActorFromClass` "/Game/Blueprints/Construction/BP_Ball.BP_Ball_C" (`SceneComponent.K2_GetComponentToWorld` (`self.Capsule`)) "AlwaysSpawn" "OverrideRootScale" null null))
  (bind _output_get (set `self.Ball` _returnvalue))
  (add `/Game/Blueprints/Construction/BP_Ball.onDead` _output_get (`|CreateDelegate` :!event `SpawnBall`))
  (return))

(fn `UserConstructionScript`)