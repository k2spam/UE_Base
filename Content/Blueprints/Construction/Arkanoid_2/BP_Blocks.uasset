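; BP_Blocks is a grid spawner that lays out a field of child actors, likely the bricks of an Arkanoid level going by its name and folder.
; Its construction script runs nested loops over X and Y, adding an auto-attached child actor component at each index multiplied by a shared Padding.
; The event graph holds only disabled stub events, so it has no runtime logic of its own.
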(fn `UserConstructionScript`
  (bind _padding (`self.Padding`))
  (for _index (range (+ (`self.X`) 1))
    (for _index_2 (range (+ (`self.Y`) 1))
      (`AddComponent|NODE_AddChildActorComponent-2` :`RelativeTransform` (`KismetMathLibrary.MakeTransform` (`KismetMathLibrary.MakeVector` (`KismetMathLibrary.Conv_IntToDouble` (* _index _padding)) (`KismetMathLibrary.Conv_IntToDouble` (* _index_2 _padding))))))))