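; BP_Wall is a temporary wall actor for the Arkanoid_2 game that appears for a limited time when triggered.
; On BeginPlay it binds to an OnShowWall dispatcher, whose event resets a countdown timer to WallTime.
; Tick decrements the timer and sets the actor's location every frame, holding it at a fixed raised position while time remains and a lowered one otherwise.
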(event `self.ReceiveBeginPlay`
  (add `self.showWall` (delegate `onShowWall`)))

(event `onShowWall`
  (set `self.Timer` (`self.Wall Time`)))

(event `self.ReceiveTick`
  (params (DeltaSeconds :type "Float (single-precision)"))
  (bind _output_get (set `self.Timer` (- (`self.Timer`) DeltaSeconds)))
  (if (> _output_get 0.0)
    (`self.K2_SetActorLocation` (-1280.0 3450.0 0.0))
    (else
      (`self.K2_SetActorLocation` (-1280.0 3450.0 -200.0)))))

(fn `UserConstructionScript`)