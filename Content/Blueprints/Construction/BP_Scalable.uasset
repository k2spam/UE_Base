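; BP_Scalable is a construction Blueprint actor that shrinks each time another actor begins overlapping it.
; After running the parent overlap handler, it skips scaling if the actor is being destroyed.
; Otherwise it reduces its current 3D scale by ScaleStep as a percentage, so repeated overlaps compound multiplicatively.
; Its construction script only calls the parent's.
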(event `self.ReceiveActorBeginOverlap`
  (params (OtherActor :type "Actor Object Reference"))
  (bind _returnvalue (`self.GetActorScale3D` self))
  (`parent.ReceiveActorBeginOverlap` OtherActor)
  (if (not (`self.IsActorBeingDestroyed`))
    (`self.SetActorScale3D` (- _returnvalue (* _returnvalue (`KismetMathLibrary.SafeDivide` (`self.Scale step`) 100.0))))))

(fn `UserConstructionScript`
  (`parent.UserConstructionScript`))