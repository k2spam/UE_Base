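; Blink light Blueprint that toggles a point light's visibility a limited number of times when play begins.
; BeginPlay runs a delayed loop with a count of twice BlinkCount, and a FlipFlop in its body alternates showing and hiding the light.
; The custom For Loop With Delay macro waits BlinkDelay before each iteration, increments a counter and loops back until the counter exceeds the count.
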(event `self.ReceiveBeginPlay`
  (bind _pointlight (`self.PointLight`))
  (`self.For Loop With Delay` (* (`self.BlinkCount`) 2) (`self.BlinkDelay`)
    (:`Body`
      (`/Engine/EditorBlueprintResources/StandardMacros.FlipFlop`
        (:`A`
          (`SceneComponent.SetVisibility` _pointlight true false))
        (:`B`
          (`SceneComponent.SetVisibility` _pointlight false false))))))

(fn `UserConstructionScript`)