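; BP_Ball is a ball actor that moves itself along a Direction vector at a given Speed and bounces off blocking surfaces.
; Each Tick it applies a swept world offset scaled by delta time.
; On a blocking hit it reflects Direction about the hit normal and cuts Speed by a tenth, never dropping below MinSpeed.
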(event `self.ReceiveTick`
  (params (DeltaSeconds :type "Float (single-precision)"))
  (bind _speed (`self.Speed`))
  (bind _minspeed (`self.MinSpeed`))
  (bind _returnvalue (- _speed (* _speed 0.1)))
  (bind _sweephitresult (`self.K2_AddActorWorldOffset` (* (* (`self.Direction`) (`self.Speed`)) DeltaSeconds) true))
  (bind (_bblockinghit _binitialoverlap _time _distance _location _impactpoint _normal) (`GameplayStatics.BreakHitResult` _sweephitresult))
  (if _bblockinghit
    (set `self.Direction` (`KismetMathLibrary.GetReflectionVector` (`self.Direction`) _normal))
    (if (>= _returnvalue _minspeed)
      (set `self.Speed` _returnvalue)
      (else
        (set `self.Speed` _minspeed)))))

(fn `UserConstructionScript`)